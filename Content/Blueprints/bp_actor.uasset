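; An actor that travels along a spline path in the level, following both its position and rotation.
; On BeginPlay it finds the Bp_path actor, stores it, and starts movement.
; A timeline alpha is lerped over the spline length to sample the world transform each update and apply it to the actor.
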(event `StartMoving`
  (bind (_direction _aplha) (`Timeline|Timeline`)
    (:`Update`
      (bind (_returnvalue_location _returnvalue_rotation) (`KismetMathLibrary.BreakTransform` (`SplineComponent.GetTransformAtDistanceAlongSpline` (`/Game/Blueprints/bp_path.Spline` (`self.Path`)) (`KismetMathLibrary.Lerp` 0.0 (`SplineComponent.GetSplineLength` (`/Game/Blueprints/bp_path.Spline` (`self.Path`))) _aplha) "World" false)))
      (`self.K2_SetActorLocationAndRotation` _returnvalue_location _returnvalue_rotation))))

(event `self.ReceiveBeginPlay`
  (bind _returnvalue (`GameplayStatics.GetActorOfClass` "/Game/Blueprints/bp_path.bp_path_C"))
  (set `self.Path` _returnvalue)
  (`self.StartMoving`))

(fn `UserConstructionScript`)